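; Enemy Blueprint for the FPS game that routes damage to a health component and hides its mesh when that component's TakeDamage returns true.
; The static mesh is supplied through Init, and Reset makes it visible again and refills health through the shared Enabled function.
; Both branches of Enabled set collision to QueryAndPhysics, so a hidden enemy keeps its collision.
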(event `self.ReceiveAnyDamage`
  (params (Damage :type "Float (single-precision)") (DamageType :type "DamageType Object Reference") (InstigatedBy :type "Controller Object Reference") (DamageCauser :type "Actor Object Reference"))
  (`self.TakeDamage` Damage))

(fn `Enabled`
  (params (IsEnabled :type Boolean) (PrimitiveComponent :type "PrimitiveComponent Object Reference"))
  (`SceneComponent.SetVisibility` PrimitiveComponent IsEnabled false)
  (if IsEnabled
    (`PrimitiveComponent.SetCollisionEnabled` PrimitiveComponent "QueryAndPhysics")
    (`/Game/FPS/Blueprints/AC_HealthComponent.SetHealthToFull` (`self.AC_HealthComponent`))
    (else
      (`PrimitiveComponent.SetCollisionEnabled` PrimitiveComponent "QueryAndPhysics"))))

(fn `Init`
  (params (StaticEnemyMesh :type "PrimitiveComponent Object Reference"))
  (set `self.StaticEnemyMesh` StaticEnemyMesh))

(fn `Reset`
  (`self.Enabled` true (`self.StaticEnemyMesh`)))

(fn `TakeDamage`
  (params (Damage :type "Float (double-precision)"))
  (returns (IsDead :type Boolean))
  (bind _isdead (`/Game/FPS/Blueprints/AC_HealthComponent.TakeDamage` (`self.AC_HealthComponent`) Damage))
  (if _isdead
    (`self.Enabled` false (`self.StaticEnemyMesh`)))
  (return _isdead))

(fn `UserConstructionScript`)