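; AC_HealthComponent is an FPS actor component that tracks an owner's health.
; It fills Health to MaxHealth on BeginPlay.
; TakeDamage caps each hit at MaxDamage, clamps Health between zero and MaxHealth, and returns whether the owner is dead via IsDead.
; GetNormalizedHealth exposes health as a zero-to-one ratio.
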(event `self.ReceiveBeginPlay`
  (`self.SetHealthToFull`))

(fn `GetNormalizedHealth`
  (returns (NormalizedHealth :type "Float (double-precision)"))
  (return (`KismetMathLibrary.FClamp` (/ (`self.Health`) (`self.MaxHealth`)))))

(fn `IsDead`
  (returns (IsDead :type Boolean))
  (return (<= (`self.Health`) 0.0)))

(fn `SetHealthToFull`
  (set `self.Health` (`self.MaxHealth`)))

(fn `TakeDamage`
  (params (Damage :type "Float (double-precision)"))
  (returns (IsDead :type Boolean))
  (bind _output_get (set `self.Health` (- (`self.Health`) (`KismetMathLibrary.FClamp` Damage 0.0 (`self.MaxDamage`)))))
  (set `self.Health` (`KismetMathLibrary.FClamp` _output_get 0.0 (`self.MaxHealth`)))
  (return (`self.IsDead`)))