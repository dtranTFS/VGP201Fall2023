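; FPS game mode Blueprint that sets up the player HUD and tracks the score.
; On BeginPlay it prints a debug start message, adds the reticle and game UI widgets to the viewport, then initializes the health bar to full and displays the current score.
; AddScore increases the stored score and pushes the new value to the game UI widget.
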(event `self.ReceiveBeginPlay`
  (`KismetSystemLibrary.PrintString` "FPSMap Starting!" true true (struct :`R` 1.0 :`A` 1.0) 5.0)
  (bind _returnvalue (`|CreateWidget` "/Game/FPS/GUI/WBP_Reticle.WBP_Reticle_C"))
  (`UserWidget.AddToViewport` _returnvalue 0)
  (bind _returnvalue_2 (`|CreateWidget` "/Game/FPS/GUI/WBP_GameUI.WBP_GameUI_C"))
  (bind _output_get (set `self.GameUI` _returnvalue_2))
  (`UserWidget.AddToViewport` _output_get 0)
  (`/Game/FPS/GUI/WBP_GameUI.SetHealthBar` _output_get 1.0)
  (`/Game/FPS/GUI/WBP_GameUI.SetScore` _output_get (`self.Score`)))

(fn `AddScore`
  (params (Points :type Integer))
  (bind _output_get (set `self.Score` (+ (`self.Score`) Points)))
  (`/Game/FPS/GUI/WBP_GameUI.SetScore` (`self.GameUI`) _output_get))

(fn `UserConstructionScript`)